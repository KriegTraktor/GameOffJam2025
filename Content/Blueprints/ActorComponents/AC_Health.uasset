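; Actor component that tracks an actor's health, applying damage, passive regeneration and death.
; Damage and regen ticks feed HealthChanged, which notifies listeners and calls Death at zero health, clearing damage and regen flags.
; Otherwise, any change, including regen ticks, clears the looping regen timer and restarts it after a retriggerable delay.
; BeginPlay caches the GameInstance and briefly delays setup to avoid a race condition.
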(event Custom|InitiateHealthRegen
  (bind _returnvalue (Utilities|Time|SetTimerbyEvent (delegate Custom|DoHealthRegen) (Variables|Default|GetHealthRegenIntervalsPerSec) true)))

(event Custom|DoHealthRegen
  (CallFunction|HealthRegenTick))

(event Custom|ResetHealthRegenDelay
  ;[0.15 0.15 0.15 0.5] When an event that causes a delay in health regen, such as taking damage, reset the delay for health regen.
  (Variables|Default|SetCanRegen false)
  (Utilities|Time|ClearandInvalidateTimerbyHandle (stale Custom|InitiateHealthRegen _returnvalue))
  (Utilities|FlowControl|RetriggerableDelay 3.0)
  (Variables|Default|SetCanRegen true)
  (CallFunction|InitiateHealthRegen))

(event Custom|ConductInitialHealthSetups
  (CallFunction|InitiateHealthRegen)
  (CallFunction|HealthChanged false))

(event EventBeginPlay
  ;[0.15 0.15 0.15 0.5] (Krieg) On BeginPlay, get a reference game GameInstance and Initialize health. Delay is necessary to prevent race condition
  (bind _asbp_game_instance (Utilities|Casting|CastToBP_GameInstance (Game|GetGameInstance)))
  (Variables|Default|SetGameInstance _asbp_game_instance)
  (Utilities|FlowControl|Delay 0.02)
  (CallFunction|ConductInitialHealthSetups))

(fn HealthChanged
  (params (TookDamage? :type Boolean))
  (if TookDamage?
    _
    (else
      _))
  ;[0.15 0.15 0.15 0.5] (Krieg) Is the actor's health <= 0?
  (if (<= (Variables|Default|GetCurrentHealth) 0.0)
    ;[0.15 0.15 0.15 0.5] (Krieg) If so, call all necessary logic to handle death
    (CallFunction|Death)
    (else
      (CallFunction|ResetHealthRegenDelay)))
  ;[0.15 0.15 0.15 0.5] (Krieg) Tell any listeners that the actor's health has changed
  (Default|CallOnHealthChanged))

(fn Death
  (Variables|Default|SetCanTakeDamage false)
  (Variables|Default|SetCanRegen false)
  (Default|CallOnDeath))

(fn HealthRegenTick
  (Variables|Default|GetCanRegen
    (:then
      (Variables|Default|SetCurrentHealth (Math|Float|Clamp(Float) (+ (Variables|Default|GetCurrentHealth) (* (Variables|Default|GetHealthRegenPerSec) (Variables|Default|GetHealthRegenIntervalsPerSec))) 0.0 (Variables|Default|GetMaxHealth)))
      (CallFunction|HealthChanged false))
    (:else)))

(fn TakeDamage
  (params (DamageAmount :type Float%20%28double-precision%29))
  (Variables|Default|SetCurrentHealth (- (Variables|Default|GetCurrentHealth) DamageAmount))
  (CallFunction|HealthChanged true)
  (Development|PrintString (Utilities|String|Append "AC_Health --- Applied damage to " (Utilities|GetDisplayName (Components|GetOwner)))))

(fn ResetStatus
  (Variables|Default|SetCurrentHealth (Variables|Default|GetMaxHealth))
  (Variables|Default|SetCanTakeDamage false)
  (Variables|Default|SetCanRegen false))