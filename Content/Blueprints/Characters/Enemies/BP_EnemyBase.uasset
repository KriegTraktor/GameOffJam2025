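; Base enemy character built for reuse after death rather than destruction.
; When its health component reports death, it ragdolls, limits capsule collision to static world and calls EnemyDeath.
; After a delay it restores physics, collision, mesh placement and health, moves to a random position, calls MakeEnemyAvailable and is unpossessed.
; Possession and unpossession toggle its HasController and InUse flags.
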(event OnDeath(AC_Health)
  (CallFunction|HandleRagdollandDisableCollision)
  (Default|CallEnemyDeath)
  (Utilities|FlowControl|Delay 5.0)
  (CallFunction|ResetEnemyforReuse)
  (Default|CallMakeEnemyAvailable)
  (Pawn|UnPossess (Pawn|GetController)))

(event EventPossessed
  (params (NewController :type Controller%20Object%20Reference))
  (Variables|Default|SetHasController true)
  (Variables|Default|SetInUse true))

(event EventUnpossessed
  (params (OldController :type Controller%20Object%20Reference))
  (Variables|Default|SetHasController false)
  (Variables|Default|SetInUse false))

(fn ConstructionScript
  (|CallParentFunction))

(fn HandleRagdollandDisableCollision
  (bind _capsulecomponent (Variables|Default|GetCapsuleComponent))
  (Physics|SetSimulatePhysics (Variables|Character|GetMesh) true)
  (Collision|SetCollisionResponsetoAllChannels _capsulecomponent "ECR_Ignore")
  (Collision|SetCollisionResponsetoChannel _capsulecomponent "ECC_WorldStatic" "ECR_Block"))

(fn ResetEnemyforReuse
  (Physics|SetSimulatePhysics (Variables|Character|GetMesh) false)
  (Collision|SetCollisionResponsetoAllChannels (Variables|Default|GetCapsuleComponent) "ECR_Block")
  (Transformation|SetWorldLocationAndRotation (Variables|Character|GetMesh) (+ (Transformation|GetWorldLocation (Variables|Default|GetCapsuleComponent)) "-20.000000,0.000000,-96.000000") "0.000000,-90.000000,0.000000" false false)
  (Transformation|SetActorLocation (Math|Vector|MakeVector (Math|Random|RandomFloatinRange -2e+03 2e+03) (Math|Random|RandomFloatinRange -2e+03 2e+03) 0.0) false false)
  (Default|ResetStatus (Variables|Default|GetAC_Health)))