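; GM_PlayMode is the play-mode game mode that links the lighthouse's health to the player's HUD.
; On BeginPlay it finds and caches the enemy manager, first-person player controller and lighthouse by class.
; It binds to the lighthouse's OnHealthChanged event, which pushes current and max health into the wave stats health bar through the controller's HUD container.
; The cached enemy manager reference is not used yet.
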(event Custom|BindEvents
  ;[0.15 0.15 0.15 0.5] (Krieg) OnHealthChanged, update the player's HUD to reflect the correct HP of the lighthouse
  (EventDispatchers|BindEventtoOnHealthChanged (Variables|Default|GetLighthouse) (delegate Custom|UpdateLighthouseHealthUI)))

(event Custom|UpdateLighthouseHealthUI
  (bind _lighthouse (Variables|Default|GetLighthouse))
  ;[0.15 0.15 0.15 0.5] (Krieg) OnHealthChanged, update the player's HUD to reflect the correct HP of the lighthouse
  (Default|UpdateHealthBar (Variables|/Game/UI/PlayerHUD/WBP_PlayerHudContainer.WBP_PlayerHudContainer_C|GetWBP_WaveStats (Variables|/Game/Blueprints/Characters/Player/PC_FirstPersonPlayer.PC_FirstPersonPlayer_C|GetWBP_PlayerHudContainer (Variables|Default|GetPlayerController))) (Variables|/Game/Blueprints/Environment/Lighthouse/BP_Lighthouse.BP_Lighthouse_C|GetCurrentHealth _lighthouse) (Variables|/Game/Blueprints/Environment/Lighthouse/BP_Lighthouse.BP_Lighthouse_C|GetMaxHealth _lighthouse)))

(event EventBeginPlay
  (bind _returnvalue (Actor|GetActorOfClass "/Game/Blueprints/Characters/Enemies/BP_EnemyManager.BP_EnemyManager_C"))
  (Variables|Default|SetEnemyManager _returnvalue)
  (bind _returnvalue_2 (Actor|GetActorOfClass "/Game/Blueprints/Characters/Player/PC_FirstPersonPlayer.PC_FirstPersonPlayer_C"))
  (Variables|Default|SetPlayerController _returnvalue_2)
  (bind _returnvalue_3 (Actor|GetActorOfClass "/Game/Blueprints/Environment/Lighthouse/BP_Lighthouse.BP_Lighthouse_C"))
  (Variables|Default|SetLighthouse _returnvalue_3)
  (CallFunction|BindEvents))

(fn ConstructionScript)